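; Player shooter character Blueprint that adds a minimap to the screen and lets the player switch cameras.
; On BeginPlay it shows the mouse cursor and creates the WB_MiniMap widget in the viewport.
; The SwitchCam input uses a FlipFlop to alternate the active camera between FirstpersonCam and Camera, enabling controller yaw rotation in both modes.
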(event Collision|EventActorBeginOverlap
  (params (OtherActor :type Actor%20Object%20Reference))
  (|CallParentFunction OtherActor) ; This node is disabled and will not be called.\nDrag off pins to build functionality.
)

(event EventTick
  (params (DeltaSeconds :type Float%20%28single-precision%29))
  (|CallParentFunction DeltaSeconds) ; This node is disabled and will not be called.\nDrag off pins to build functionality.
)

(event EventBeginPlay
  (bind _returnvalue (Game|GetPlayerController 0))
  (Variables|/Script/Engine.PlayerController|SetbShowMouseCursor _returnvalue true)
  (bind _returnvalue_2 (UserInterface|CreateWidget "/Game/UI/WB_MiniMap.WB_MiniMap_C" _returnvalue))
  (UserInterface|Viewport|AddtoViewport _returnvalue_2 0))

(event Input|ActionEvents|InputActionSwitchCam
  (params (Key :type Key%20Structure :default "None"))
  (:Pressed
    (Utilities|FlowControl|FlipFlop
      (:A
        (Components|Activation|SetActive (Variables|Default|GetFirstpersonCam) true false)
        (Components|Activation|SetActive (Variables|Default|GetCamera) false false)
        (Variables|Default|SetbUseControllerRotationYaw true))
      (:B
        (Components|Activation|SetActive (Variables|Default|GetFirstpersonCam) false false)
        (Components|Activation|SetActive (Variables|Default|GetCamera) true false)
        (Variables|Default|SetbUseControllerRotationYaw true)))))

(fn ConstructionScript
  (|CallParentFunction))